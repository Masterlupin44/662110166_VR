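; CubeTimeline_BP is an actor that slides its Cube component from its starting world location to TargetLocation.
; On BeginPlay it caches the cube's position, waits briefly, then plays a timeline whose track drives a vector lerp.
; When that timeline finishes it only zeroes SelfLocation2.
; A matching second timeline for Cube2 is never triggered, so that cube is not moved.
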(event Collision|EventActorBeginOverlap
  (params (OtherActor :type Actor%20Object%20Reference)))

(event EventTick
  (params (DeltaSeconds :type Float%20%28single-precision%29)))

(event EventBeginPlay
  (Variables|Default|SetSelf%20Location (Transformation|GetWorldLocation (Variables|Default|GetCube)))
  (Utilities|FlowControl|Delay 2.0)
  (bind _time (Timeline|Timeline PlayFromStart)
    (:Update
      (Transformation|SetWorldLocation (Variables|Default|GetCube) (Math|Vector|Lerp(Vector) (Variables|Default|GetSelf%20Location) (Variables|Default|GetTarget%20Location) _time) false false))
    (:Finished
      (Variables|Default|SetSelf%20Location_2 "0, 0, 0"))))

(fn ConstructionScript)